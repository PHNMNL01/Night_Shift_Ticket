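; BP_PC_TicketInteractable is an interactable PC that shows a ticket text widget on screen when the player uses it.
; It creates the WBPTicketText widget once at BeginPlay and enables input only while the player pawn is inside InteractZone.
; E toggles the widget in the viewport and Q closes it; leaving the zone also closes it and disables input, with debug prints on enter and exit.
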(event `self.ReceiveBeginPlay`
  (bind _returnvalue (`|CreateWidget` (`self.WBP_TicketText`) (`GameplayStatics.GetPlayerController` 0)))
  (set `self.TicketWidgetRef` _returnvalue)
  (set `self.bTicketOpen` false))

(event `Key|E`
  (params (Key :type "Key Structure"))
  (bind _ticketwidgetref (`self.TicketWidgetRef`))
  (:`Pressed`
    (if (`self.bPlayerInRange`)
      (if (`self.bTicketOpen`)
        (`self.CloseTicket`)
        (else
          (`/Engine/EditorBlueprintResources/StandardMacros.IsValid` _ticketwidgetref
            (:`Is Valid`
              (`UserWidget.AddToViewport` _ticketwidgetref 10)
              (set `self.bTicketOpen` true))))))))

(event `CloseTicket`
  (bind _ticketwidgetref (`self.TicketWidgetRef`))
  (`/Engine/EditorBlueprintResources/StandardMacros.IsValid` _ticketwidgetref
    (:`Is Valid`
      (`Widget.RemoveFromParent` _ticketwidgetref))
    (:`Is Not Valid`
      _))
  (set `self.bTicketOpen` false))

(event `Key|Q`
  (params (Key :type "Key Structure"))
  (:`Pressed`
    (if (`self.bTicketOpen`)
      (`self.CloseTicket`))))

(event `self.InteractZone.OnComponentBeginOverlap`
  (params (OverlappedComponent :type "PrimitiveComponent Object Reference") (OtherActor :type "Actor Object Reference") (OtherComp :type "PrimitiveComponent Object Reference") (OtherBodyIndex :type Integer) (bFromSweep :type Boolean) (SweepResult :type "HitResult Structure (by ref)"))
  (if (== OtherActor (`GameplayStatics.GetPlayerPawn` 0))
    (set `self.bPlayerInRange` true)
    (`self.EnableInput` (`GameplayStatics.GetPlayerController` 0))
    (`KismetSystemLibrary.PrintString` "Press E")))

(event `self.InteractZone.OnComponentEndOverlap`
  (params (OverlappedComponent :type "PrimitiveComponent Object Reference") (OtherActor :type "Actor Object Reference") (OtherComp :type "PrimitiveComponent Object Reference") (OtherBodyIndex :type Integer))
  (if (== OtherActor (`GameplayStatics.GetPlayerPawn` 0))
    (set `self.bPlayerInRange` false)
    (`self.CloseTicket`)
    (`self.DisableInput` (`GameplayStatics.GetPlayerController` 0))
    (`KismetSystemLibrary.PrintString` "PLayer left PC")))

(fn `UserConstructionScript`)