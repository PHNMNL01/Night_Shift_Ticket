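; Horror event director that triggers a one-time chandelier fall after the player captures evidence.
; On BeginPlay it binds to the first-person character's OnEvidenceCaptured dispatcher.
; The first capture arms the sequence, waits a configurable delay, then calls TriggerFall on a referenced chandelier.
; A flag blocks repeat triggers, and debug prints report a failed player cast or missing chandelier reference.
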(event `self.ReceiveBeginPlay`
  (bind _asbp_first_person_character (cast `/Game/FirstPerson/Blueprints/BP_FirstPersonCharacter` (`GameplayStatics.GetPlayerCharacter` 0))
    (:`then`
      (add `/Game/FirstPerson/Blueprints/BP_FirstPersonCharacter.OnEvidenceCaptured` _asbp_first_person_character (delegate `HandleEvidenceCaptured`)))
    (:`CastFailed`
      (`KismetSystemLibrary.PrintString` "HORROR DIRECTOR: PLAYER CAST FAILED"))))

(event `HandleEvidenceCaptured`
  (if (not (`self.bSequenceArmed`))
    (set `self.bSequenceArmed` true)
    (`KismetSystemLibrary.PrintString` "HORROR SEQUENCE ARMED")
    (`KismetSystemLibrary.Delay` (`self.ChandelierDelay`))
    (`/Engine/EditorBlueprintResources/StandardMacros.IsValid` (`self.ChandelierRef`)
      (:`Is Valid`
        (`/Game/HorrorEvents/BP_Chandelier.TriggerFall` (`self.ChandelierRef`)))
      (:`Is Not Valid`
        (`KismetSystemLibrary.PrintString` "HORROR DIRECTOR: CHANDELIER REF MISSING")))))

(fn `UserConstructionScript`)