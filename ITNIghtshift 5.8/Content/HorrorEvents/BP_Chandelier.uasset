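; BP_Chandelier is a horror event actor that drops a chandelier a set distance straight down, once.
; BeginPlay caches the start and target locations from DropDistance, and an optional test flag triggers the fall after a short delay.
; TriggerFall is guarded against repeats and plays a timeline that lerps the actor between those locations without sweep or physics, printing a debug message on landing.
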(event `self.ReceiveBeginPlay`
  (bind _returnvalue (`self.K2_GetActorLocation`))
  (set `self.StartLocation` _returnvalue)
  (set `self.TargetLocation` (+ _returnvalue (`KismetMathLibrary.MakeVector` 0.0 0.0 (- 0.0 (`self.DropDistance`)))))
  (if (`self.bTestFallOnBeginPlay`)
    (`KismetSystemLibrary.Delay` 2.0)
    (`self.TriggerFall`)))

(event `TriggerFall`
  (if (not (`self.bHasFallen`))
    (set `self.bHasFallen` true)
    (bind (_direction _alpha) (`Timeline|TL_ChandelierFall`)
      (:`Update`
        (`self.K2_SetActorLocation` self (`KismetMathLibrary.VLerp` (`self.StartLocation`) (`self.TargetLocation`) _alpha) false false))
      (:`Finished`
        (`KismetSystemLibrary.PrintString` "CHANDELIER LANDED")))))

(fn `UserConstructionScript`)